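; AC_Health is a health component that tracks current health, maximum health and a death state for its owner.
; Events to reset, gain or take damage all route through UpdateHealthAndNotify, with gain and damage ignored once dead.
; That function clamps health between zero and MaxHealth, calls OnHealthChanged, then sets IsDead and calls OnDeath at zero.
; ResetHealth clears the death state and restores full health.
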(event EventResetHealth
  (Variables|Default|SetIsDead false)
  (CallFunction|UpdateHealthandNotify (Variables|Default|GetMaxHealth)))

(event EventGainHealth
  (params (HealthAmount :type Float%20%28double-precision%29))
  (if (not (Variables|Default|GetIsDead))
    (CallFunction|UpdateHealthandNotify (+ (Variables|Default|GetCurrentHealth) HealthAmount))))

(event EventTakeDamage
  (params (DamageAmount :type Float%20%28double-precision%29))
  (if (not (Variables|Default|GetIsDead))
    (CallFunction|UpdateHealthandNotify (- (Variables|Default|GetCurrentHealth) DamageAmount))))

(fn UpdateHealthandNotify
  (params (NewHealth :type Float%20%28double-precision%29))
  ;[0.15 0.15 0.15 0.5] HILT HILTH HILTH HILTH
  (bind _output_get (Variables|Default|SetCurrentHealth (Math|Float|Clamp(Float) NewHealth 0.0 (Variables|Default|GetMaxHealth))))
  (Default|CallOnHealthChanged _output_get (Variables|Default|GetMaxHealth))
  (if (<= (Variables|Default|GetCurrentHealth) 0.0)
    (Variables|Default|SetIsDead true)
    (Default|CallOnDeath)
    (else
      (Variables|Default|SetIsDead false))))